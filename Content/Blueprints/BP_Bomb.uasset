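; BP_Bomb is a falling bomb that destroys any BP_Person it hits.
; Each Tick teleports it down by a fixed step, so fall speed depends on frame rate.
; A CollSphere overlap with a person spawns an explosion emitter and destroys both actors.
; If it drops below a height threshold, it spawns the same emitter above its position and destroys itself.
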(event OnComponentBeginOverlap(CollSphere)
  (params (OverlappedComponent :type Primitive%20Component%20Object%20Reference) (OtherActor :type Actor%20Object%20Reference) (OtherComp :type Primitive%20Component%20Object%20Reference) (OtherBodyIndex :type Integer) (bFromSweep :type Boolean) (SweepResult :type Hit%20Result%20Structure%20%28by%20ref%29))
  (bind _asbp_person (Utilities|Casting|CastToBP_Person OtherActor))
  (Effects|SpawnEmitteratLocation "/Engine/Tutorial/SubEditors/TutorialAssets/TutorialParticleSystem.TutorialParticleSystem" (Transformation|GetActorLocation) "0, 0, 0" "5.000000,5.000000,5.000000")
  (Actor|DestroyActor _asbp_person)
  (Actor|DestroyActor))

(event EventBeginPlay)

(event Collision|EventActorBeginOverlap
  (params (OtherActor :type Actor%20Object%20Reference)))

(event EventTick
  (params (DeltaSeconds :type Float%20%28single-precision%29))
  (bind _returnvalue (Transformation|GetActorLocation))
  (bind _returnvalue_2 (Transformation|GetActorLocation))
  (Transformation|Teleport (Math|Vector|MakeVector (.x _returnvalue) (.y _returnvalue) (- (.z _returnvalue) 5e+01)) "0, 0, 0")
  (if (< (.z (.location (Transformation|GetActorTransform))) -5e+02)
    (Effects|SpawnEmitteratLocation "/Engine/Tutorial/SubEditors/TutorialAssets/TutorialParticleSystem.TutorialParticleSystem" (Math|Vector|MakeVector (.x _returnvalue_2) (.y _returnvalue_2) (+ (.z _returnvalue_2) 5e+02)) "0, 0, 0" "5.000000,5.000000,5.000000")
    (Actor|DestroyActor)))

(fn ConstructionScript)